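; Game mode that keeps spawning jump platforms throughout play.
; BeginPlay starts a looping timer that calls CreatePlatform, which spawns a BP_JumpPlatform at the world origin with a random sideways offset along Y.
; A RandomPlatform helper picks either BP_Platform or a random PlatformList entry, but the spawn logic does not use it.
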(event `self.ReceiveBeginPlay`
  (`KismetSystemLibrary.K2_SetTimer` null "CreatePlatform" 1.5 true))

(fn `CreatePlatform`
  (`|SpawnActorFromClass` "/Game/Blueprints/Platform/BP_JumpPlatform.BP_JumpPlatform_C" (`KismetMathLibrary.Conv_VectorToTransform` (`KismetMathLibrary.MakeVector` 0.0 (* (`KismetMathLibrary.RandomFloatInRange` -1.0 1.0) 600.0))) "Undefined" "MultiplyWithRoot" null null))

(fn `RandomPlatform`
  (returns (Result :type "/Game/Blueprints/Platform/BP_Platform Class Reference"))
  (if (`KismetMathLibrary.RandomBool`)
    (return "/Game/Blueprints/Platform/BP_Platform.BP_Platform_C")
    (else
      (return (`KismetArrayLibrary.Array_Random` (`self.PlatformList`))))))

(fn `UserConstructionScript`)