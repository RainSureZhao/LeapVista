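; BP_PickableItem is a pickup item that moves along Z and is collected when the player character touches it.
; On BeginPlay it sets its ProjectileMovement vertical velocity from MyGameMode's Count plus a base speed, so higher counts give a higher Z velocity.
; Overlap with BP_MyCharacter calls PickUp, which is empty here, then destroys the actor.
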(event `self.ReceiveBeginPlay`
  (bind _asmy_game_mode (cast `/Game/Blueprints/MyGameMode` (`GameplayStatics.GetGameMode`)))
  (set `MovementComponent.Velocity` (`KismetMathLibrary.MakeVector` 0.0 0.0 (+ (/ (`/Game/Blueprints/MyGameMode.Count` _asmy_game_mode) 2.0) 150.0)) (`self.ProjectileMovement`)))

(event `self.ReceiveActorBeginOverlap`
  (params (OtherActor :type "Actor Object Reference"))
  (cast `/Game/Blueprints/Player/BP_MyCharacter` OtherActor)
  (`self.PickUp`)
  (`self.K2_DestroyActor`))

(fn `PickUp`)

(fn `UserConstructionScript`)