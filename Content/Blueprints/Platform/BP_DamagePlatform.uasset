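; BP_DamagePlatform is a platform that hurts the player and bounces them upward.
; Any actor overlap triggers it, acting on player 0's BP_MyCharacter without checking the overlapping actor.
; It clears vertical velocity, adds upward movement and removes one health.
; It also raises the "die" scalar in the MP_Die parameter collection, then a half-second timer resets it to zero.
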(event `self.ReceiveBeginPlay`
  (`parent.ReceiveBeginPlay`))

(event `self.ReceiveActorBeginOverlap`
  (params (OtherActor :type "Actor Object Reference"))
  (`parent.ReceiveActorBeginOverlap` OtherActor)
  (bind _asbp_my_character (cast `/Game/Blueprints/Player/BP_MyCharacter` (`GameplayStatics.GetPlayerCharacter` 0)))
  (`/Game/Blueprints/Player/BP_MyCharacter.ClearVelocityZ` _asbp_my_character)
  (`/Game/Blueprints/Player/BP_MyCharacter.AddMovement` _asbp_my_character (0.0 0.0 500.0))
  (`/Game/Blueprints/Player/BP_MyCharacter.ChangeHealth` _asbp_my_character -1)
  (`KismetMaterialLibrary.SetScalarParameterValue` "/Game/Materials/MP_Die.MP_Die" "die" 0.5)
  (`KismetSystemLibrary.K2_SetTimerDelegate` (delegate `CustomEvent`) 0.5))

(event `CustomEvent`
  (`KismetMaterialLibrary.SetScalarParameterValue` "/Game/Materials/MP_Die.MP_Die" "die" 0.0))

(event `self.Box.OnComponentBeginOverlap`
  (params (OverlappedComponent :type "PrimitiveComponent Object Reference") (OtherActor :type "Actor Object Reference") (OtherComp :type "PrimitiveComponent Object Reference") (OtherBodyIndex :type Integer) (bFromSweep :type Boolean) (SweepResult :type "HitResult Structure (by ref)")))

(fn `UserConstructionScript`
  (`parent.UserConstructionScript`))