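; MyPlayerState is a player state Blueprint that holds the player's health and energy.
; On BeginPlay it binds to the first player's BP_MyCharacter change-health event, which feeds a function that clamps health between zero and MaxHealth.
; When health reaches zero it calls GameOver on MyGameMode.
; A separate ChangeEnergy function clamps energy the same way, though nothing in this graph calls it.
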(event `self.ReceiveBeginPlay`
  (bind _asbp_my_character (cast `/Game/Blueprints/Player/BP_MyCharacter` (`GameplayStatics.GetPlayerCharacter` 0)))
  (add `/Game/Blueprints/Player/BP_MyCharacter.ChangeHealth` _asbp_my_character (delegate `CustomEvent`)))

(event `CustomEvent`
  (params (Count :type Integer))
  (`self.ChangeHealth` Count))

(fn `ChangeEnergy`
  (params (Count :type Integer))
  (set `self.Energy` (`KismetMathLibrary.Clamp` (+ Count (`self.Energy`)) 0 (`self.MaxEnergy`))))

(fn `ChangeHealth`
  (params (Count :type Integer))
  (`|ExecutionSequence`
    (:`then_0`
      (set `self.Health` (`KismetMathLibrary.Clamp` (+ (`self.Health`) Count) 0 (`self.MaxHealth`))))
    (:`then_1`
      (if (== (`self.Health`) 0)
        (bind _asmy_game_mode (cast `/Game/Blueprints/MyGameMode` (`GameplayStatics.GetGameMode`)))
        (`/Game/Blueprints/MyGameMode.GameOver` _asmy_game_mode)))))

(fn `UserConstructionScript`)